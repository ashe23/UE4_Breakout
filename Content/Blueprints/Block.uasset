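; Block is a destructible actor that awards score when hit.
; On Hit it plays a pop sound at the hit location, destroys itself, then adds points to the score and decrements the block count on MainGameMode.
; The construction script creates a dynamic material instance from M_Base and sets its Color parameter from the block's Color variable, so each block can be tinted individually.
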(event Collision|EventHit
  (params (MyComp :type Primitive%20Component%20Object%20Reference) (Other :type Actor%20Object%20Reference) (OtherComp :type Primitive%20Component%20Object%20Reference) (bSelfMoved :type Boolean) (HitLocation :type Vector) (HitNormal :type Vector :default "0, 0, 0") (NormalImpulse :type Vector :default "0, 0, 0") (Hit :type Hit%20Result%20Structure%20%28by%20ref%29))
  (Audio|PlaySoundatLocation "/Game/Audio/pop.pop" HitLocation)
  (Actor|DestroyActor)
  (bind _asmain_game_mode (Utilities|Casting|CastToMainGameMode (Game|GetGameMode)))
  (Variables|Default|SetGameMode _asmain_game_mode)
  (Variables|/Game/Blueprints/MainGameMode.MainGameMode_C|SetScore (Variables|Default|GetGameMode) (+ (Variables|/Game/Blueprints/MainGameMode.MainGameMode_C|GetScore (Variables|Default|GetGameMode)) 100))
  (Variables|/Game/Blueprints/MainGameMode.MainGameMode_C|SetBlockCount (Variables|Default|GetGameMode) (- (Variables|/Game/Blueprints/MainGameMode.MainGameMode_C|GetBlockCount (Variables|Default|GetGameMode)) 1)))

(fn ConstructionScript
  (bind _returnvalue (Rendering|Material|CreateDynamicMaterialInstance "/Game/Materials/M_Base.M_Base" :!class /Script/Engine.KismetMaterialLibrary))
  (Rendering|Material|SetVectorParameterValue _returnvalue "Color" (Variables|Default|GetColor) :!class /Script/Engine.MaterialInstanceDynamic))