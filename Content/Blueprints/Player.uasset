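; Player pawn for a paddle-and-ball game that moves the paddle and launches balls.
; Tick applies force to the Paddle along X from horizontal input and Speed.
; Fire and SpawnNewBall duplicate the same spawn of a scaled-up Ball at the pawn with randomized yaw, while SpawnBall uses BallFireDirection and prints a debug string.
; Menu input opens the pause menu through the cached MainGameMode, and Quit exits the game.
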(event Custom|SpawnBall
  (Game|SpawnActorfromClass "/Game/Blueprints/Ball.Ball_C" (Transformation|GetWorldTransform (Variables|Default|GetBallFireDirection)) "Undefined" 0 0)
  (Development|PrintString "Hello"))

(event Custom|SpawnNewBall
  (bind _returnvalue (Game|Player|GetPlayerPawn 0))
  (bind _returnvalue_2 (Transformation|GetActorTransform _returnvalue))
  ;[1 1 1] Spawns ball with random color and direction
  (Game|SpawnActorfromClass "/Game/Blueprints/Ball.Ball_C" (Math|Transform|MakeTransform (.location _returnvalue_2) (Math|Rotator|MakeRotator (.yaw (.rotation _returnvalue_2)) (.yaw (.rotation _returnvalue_2)) (Math|Random|RandomFloatinRange 1.8e+02 2.7e+02)) "2.000000,2.000000,2.000000") "Undefined" 0 0))

(event EventTick
  (params (DeltaSeconds :type Float%20%28single-precision%29))
  ;[1 1 1] Moving Paddle
  (Physics|AddForce (Variables|Default|GetPaddle) (Math|Vector|MakeVector (* (Input|AxisValues|GetMoveHorizontal) (Variables|Default|GetSpeed)) 0.0 0.0) "None" false))

(event EventBeginPlay
  (bind _asmain_game_mode (Utilities|Casting|CastToMainGameMode (Game|GetGameMode)))
  (Variables|Default|SetGameMode _asmain_game_mode))

(event Input|ActionEvents|InputActionMenu
  (params (Key :type Key%20Structure :default "AnyKey"))
  ;[1 1 1] Opens Main Menu
  (:Pressed
    (Default|OpenPauseMenu (Variables|Default|GetGameMode))))

(event Input|ActionEvents|InputActionQuit
  (params (Key :type Key%20Structure :default "AnyKey"))
  ;[1 1 1] Quit Game
  (:Pressed
    (Game|QuitGame 0 "Quit")))

(event Input|ActionEvents|InputActionFire
  (params (Key :type Key%20Structure :default "AnyKey"))
  (bind _returnvalue (Game|Player|GetPlayerPawn 0))
  (bind _returnvalue_2 (Transformation|GetActorTransform _returnvalue))
  (:Pressed
    (Game|SpawnActorfromClass "/Game/Blueprints/Ball.Ball_C" (Math|Transform|MakeTransform (.location _returnvalue_2) (Math|Rotator|MakeRotator (.yaw (.rotation _returnvalue_2)) (.yaw (.rotation _returnvalue_2)) (Math|Random|RandomFloatinRange 1.8e+02 2.7e+02)) "2.000000,2.000000,2.000000") "Undefined" 0 0)))

(fn ConstructionScript)