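; KillZone is an actor that handles a lost ball when one overlaps it.
; It caches the MainGameMode on BeginPlay.
; On overlap with a Ball, it destroys the ball, decrements the game mode's Lifes and calls SpawnNewBall on the Player pawn.
; It does no check on remaining lives before requesting the new ball.
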(event EventBeginPlay
  (bind _asmain_game_mode (Utilities|Casting|CastToMainGameMode (Game|GetGameMode)))
  (Variables|Default|SetGameMode _asmain_game_mode))

(event Collision|EventActorBeginOverlap
  (params (OtherActor :type Actor%20Object%20Reference))
  (bind _gamemode (Variables|Default|GetGameMode))
  ;[1 1 1] Destroying ball , and spawning new ball if there is life
  (bind _asball (Utilities|Casting|CastToBall OtherActor))
  (Actor|DestroyActor _asball)
  (Variables|/Game/Blueprints/MainGameMode.MainGameMode_C|SetLifes _gamemode (- (Variables|/Game/Blueprints/MainGameMode.MainGameMode_C|GetLifes _gamemode) 1))
  (bind _asplayer (Utilities|Casting|CastToPlayer (Game|Player|GetPlayerPawn 0)))
  (Default|SpawnNewBall _asplayer))

(fn ConstructionScript)