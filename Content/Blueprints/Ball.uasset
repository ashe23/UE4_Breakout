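; Physics-driven ball that moves at constant speed along diagonal headings in the horizontal plane.
; BeginPlay caches the Player pawn, then launches the ball with an impulse and randomizes its material color, overriding the construction script's Color.
; Every Tick, ClampVelocity forces velocity to Speed and snaps yaw to the nearest diagonal by rotating 45°, rounding to 90° steps and rotating back.
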(event Custom|ClampVelocity
  (bind _returnvalue (Transformation|GetVelocity))
  (bind _returnvalue_2 (Math|Rotator|MakeRotator 0.0 0.0 45.0))
  (bind _speed (Variables|Default|GetSpeed))
  (bind _returnvalue_3 (Math|Vector|ClampVectorSize _returnvalue _speed _speed))
  ;[1 1 1] Clamp ball velocity and movement angle to 45°
  (Physics|SetPhysicsLinearVelocity (Variables|Default|GetBall) (* (Math|Vector|UnrotateVector (Math|Rotator|GetRotationXVector (Math|Rotator|MakeRotator 0.0 0.0 (|((round((A/B)))*B) (.yaw (Math|Rotator|MakeRotfromX (Math|Vector|RotateVector _returnvalue_3 _returnvalue_2))) 9e+01))) _returnvalue_2) (Math|Vector|VectorLength _returnvalue_3)) false "None"))

(event EventBeginPlay
  (bind _ball (Variables|Default|GetBall))
  (bind _asplayer (Utilities|Casting|CastToPlayer (Pawn|GetControlledPawn (Game|GetPlayerController 0))))
  (Variables|Default|SetPlayer _asplayer)
  (Physics|AddImpulse _ball "-100000.000000, 0, 0" "None" false)
  (Rendering|Material|SetVectorParameterValueonMaterials _ball "Color" (Math|Vector|MakeVector (Math|Random|RandomFloatinRange 0.0 1.0) (Math|Random|RandomFloatinRange 0.0 1.0) (Math|Random|RandomFloatinRange 0.0 1.0))))

(event EventTick
  (params (DeltaSeconds :type Float%20%28single-precision%29))
  (CallFunction|ClampVelocity))

(fn ConstructionScript
  (bind _returnvalue (Rendering|Material|CreateDynamicMaterialInstance (Variables|Default|GetBall) 0 "/Game/Materials/M_Base.M_Base" :!class /Script/Engine.PrimitiveComponent))
  (Rendering|Material|SetVectorParameterValue _returnvalue "Color" (Variables|Default|GetColor) :!class /Script/Engine.MaterialInstanceDynamic))