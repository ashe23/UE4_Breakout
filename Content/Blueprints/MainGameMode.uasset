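; Game mode for a block-clearing game that tracks lives, block count and win/lose status.
; Tick polls both end conditions: zero lives loses, while zero blocks with lives remaining wins.
; Either result pauses the game, shows the shared GameOver widget and cursor, sets GameStatus and plays a sound.
; Separate events open the pause and main menus, also pausing and showing the cursor.
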(event Custom|isGameOver
  ;[1 1 1] Checks if game is over
  (if (== (Variables|Default|GetLifes) 0)
    (Audio|PlaySoundatLocation "/Game/Audio/negative.negative" "0, 0, 0")
    (Game|SetGamePaused true)
    (bind _returnvalue (UserInterface|CreateWidget "/Game/HUD/GameOver.GameOver_C"))
    (UserInterface|Viewport|AddtoViewport _returnvalue 0)
    (Variables|/Script/Engine.PlayerController|SetbShowMouseCursor (Game|GetPlayerController 0) true)
    (Variables|Default|SetGameStatus "NewEnumerator1")
    (Audio|PlaySound2D "/Game/Audio/negative.negative")))

(event Custom|isWin
  ;[1 1 1] Checks if player win
  (if (and (== (Variables|Default|GetBlockCount) 0) (!= (Variables|Default|GetLifes) 0))
    (Game|SetGamePaused true)
    (bind _returnvalue (UserInterface|CreateWidget "/Game/HUD/GameOver.GameOver_C"))
    (UserInterface|Viewport|AddtoViewport _returnvalue 0)
    (Variables|/Script/Engine.PlayerController|SetbShowMouseCursor (Game|GetPlayerController 0) true)
    (Variables|Default|SetGameStatus "NewEnumerator0")
    (Audio|PlaySound2D "/Game/Audio/positive.positive")))

(event Custom|OpenPauseMenu
  (bind _returnvalue (UserInterface|CreateWidget "/Game/HUD/PauseMenu.PauseMenu_C"))
  (Game|SetGamePaused true)
  (UserInterface|Viewport|AddtoViewport _returnvalue 0)
  (Variables|/Script/Engine.PlayerController|SetbShowMouseCursor (Game|GetPlayerController 0) true))

(event Custom|OpenMainMenu
  (bind _returnvalue (UserInterface|CreateWidget "/Game/HUD/Menu.Menu_C"))
  (UserInterface|Viewport|AddtoViewport _returnvalue 0)
  (Game|SetGamePaused true)
  (Variables|/Script/Engine.PlayerController|SetbShowMouseCursor (Game|GetPlayerController 0) true))

(event EventTick
  (params (DeltaSeconds :type Float%20%28single-precision%29))
  ;[1 1 1] Checking game status on every frame
  (CallFunction|IsGameOver)
  (CallFunction|IsWin))

(fn ConstructionScript)